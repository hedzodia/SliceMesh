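; A short-lived cutting ball actor that slices any procedural mesh it hits and destroys itself five seconds after spawning.
; On a sphere hit, it cuts the mesh at the impact point, using VectorDirection as the plane normal and capping the cut with a base material.
; The new half gets physics, both halves receive opposite velocity-change impulses to push them apart, and the ball is destroyed.
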(event OnComponentHit(Sphere1)
  (params (HitComponent :type Primitive%20Component%20Object%20Reference) (OtherActor :type Actor%20Object%20Reference) (OtherComp :type Primitive%20Component%20Object%20Reference) (NormalImpulse :type Vector :default "0, 0, 0") (Hit :type Hit%20Result%20Structure%20%28by%20ref%29))
  (bind _vectordirection (Variables|Default|GetvectorDirection))
  (bind _returnvalue (* _vectordirection 5))
  (bind _returnvalue_2 (+ _returnvalue (.normal Hit)))
  (bind _returnvalue_3 (* _returnvalue_2 200))
  (bind _asprocedural_mesh_component (Utilities|Casting|CastToProceduralMeshComponent OtherComp))
  (bind _outotherhalfprocmesh (Class|KismetProceduralMeshLibrary|SliceProceduralMesh _asprocedural_mesh_component (.location Hit) (Variables|Default|GetvectorDirection) true "CreateNewSectionForCap" "/Game/FirstPerson/Meshes/BaseMaterial.BaseMaterial"))
  (Physics|SetSimulatePhysics _outotherhalfprocmesh true)
  (Physics|AddImpulse _outotherhalfprocmesh _returnvalue_3 "None" true)
  (Physics|AddImpulse _asprocedural_mesh_component (* _returnvalue_3 -1) "None" true)
  (Actor|DestroyActor))

(event EventBeginPlay
  (Utilities|FlowControl|Delay 5.0)
  (Actor|DestroyActor))

(fn ConstructionScript)