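; Cuttable-object Blueprint, judging by its name, that turns a configurable static mesh into procedural geometry.
; The Construction Script applies the mesh and material variables to the Cube component, then sets a shared world scale on it and the ProceduralMesh.
; It copies Cube's geometry into the ProceduralMesh with collision enabled.
; The event graph is empty, so this Blueprint's graphs contain no cutting logic.
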(event EventBeginPlay)

(event Collision|EventActorBeginOverlap
  (params (OtherActor :type Actor%20Object%20Reference)))

(event EventTick
  (params (DeltaSeconds :type Float%20%28single-precision%29)))

(fn ConstructionScript
  (Components|StaticMesh|SetStaticMesh (Variables|Default|GetCube) (Variables|Default|Getmesh))
  (Rendering|Material|SetMaterial (Variables|Default|GetCube) 0 (Variables|Default|Getmat))
  (Transformation|SetWorldScale3D (Variables|Default|GetCube) (Variables|Default|Getscale))
  (Class|KismetProceduralMeshLibrary|CopyProceduralMeshfromStaticMeshComponent (Variables|Default|GetCube) 0 (Variables|Default|GetProceduralMesh) true))